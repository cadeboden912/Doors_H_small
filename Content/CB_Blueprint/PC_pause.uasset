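; PC_pause is a Blueprint, apparently a player controller, that toggles a pause menu when the pause input action is pressed.
; If no menu reference is valid, it creates and stores a MainMenu widget, adds it to the viewport, switches to Game and UI input, shows the cursor and pauses the game.
; Otherwise it removes and clears the widget, restores game-only input, unpauses and sets its own cursor flag to hidden.
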(event Input|ActionEvents|InputActionpause
  (params (Key :type Key%20Structure :default "None"))
  (bind _returnvalue (Game|GetPlayerController 0))
  (bind _returnvalue_2 (Game|GetPlayerController 0))
  (:Pressed
    (Utilities|IsValid (Variables|Default|GetPauseUiRef)
      (:Is%20Valid
        (Widget|RemovefromParent (Variables|Default|GetPauseUiRef))
        (Variables|Default|SetPauseUiRef 0)
        (Input|SetInputModeGameOnly _returnvalue_2)
        (Variables|/Script/Engine.PlayerController|SetbShowMouseCursor _returnvalue_2 true)
        (Game|SetGamePaused false)
        (Variables|Default|SetbShowMouseCursor false))
      (:Is%20Not%20Valid
        (bind _returnvalue_3 (UserInterface|CreateWidget "/Game/CB_Widgets/MainMenu.MainMenu_C"))
        (bind _output_get (Variables|Default|SetPauseUiRef _returnvalue_3))
        (UserInterface|Viewport|AddtoViewport _output_get 0)
        (Input|SetInputModeGameandUI _returnvalue 0 "DoNotLock" true)
        (Variables|/Script/Engine.PlayerController|SetbShowMouseCursor _returnvalue true)
        (Game|SetGamePaused true)))))

(fn ConstructionScript)